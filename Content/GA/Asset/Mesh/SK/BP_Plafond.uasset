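; BP_Plafond is an animated ceiling ("plafond") actor that continuously rotates six pivot components from BeginPlay.
; The Moving timeline drives the roll of four pivots set at 90-degree yaw offsets.
; Its updates also play the MOVINGROND timeline, which drives the yaw of two more pivots, one flipped upside down, and applies all six rotations.
; When either timeline finishes, both restart from the beginning, forming an endless loop.
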(event Collision|EventActorBeginOverlap
  (params (OtherActor :type Actor%20Object%20Reference)))

(event EventTick
  (params (DeltaSeconds :type Float%20%28single-precision%29)))

(event EventBeginPlay
  (bind _newtrack_0 (Timeline|moving Play)
    (:Update
      (bind _newtrack_0_2 (Timeline|MOVINGROND Play)
        (:Update
          (Transformation|SetRelativeRotation (Variables|Default|Getpivot) (Math|Rotator|MakeRotator _newtrack_0 0.0 0.0) false false)
          (Transformation|SetRelativeRotation (Variables|Default|Getpivot1) (Math|Rotator|MakeRotator _newtrack_0 0.0 1.8e+02) false false)
          (Transformation|SetRelativeRotation (Variables|Default|Getpivot2) (Math|Rotator|MakeRotator _newtrack_0 0.0 9e+01) false false)
          (Transformation|SetRelativeRotation (Variables|Default|Getpivot3) (Math|Rotator|MakeRotator _newtrack_0 0.0 -9e+01) false false)
          (Transformation|SetRelativeRotation (Variables|Default|Getpivot4) (Math|Rotator|MakeRotator 0.0 0.0 _newtrack_0_2) false false)
          (Transformation|SetRelativeRotation (Variables|Default|Getpivot5) (Math|Rotator|MakeRotator 1.8e+02 0.0 _newtrack_0_2) false false))
        (:Finished
          (for _index (range 0 0) :!label _label
            (Timeline|moving PlayFromStart))
          (Timeline|MOVINGROND PlayFromStart))))
    (:Finished
      (goto _label))))

(fn ConstructionScript)