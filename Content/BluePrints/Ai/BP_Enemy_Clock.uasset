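; BP_Enemy_Clock is a clock enemy whose eye component can turn to follow the player and swing back to rest.
; RotateEye blends the eye toward a look-at rotation, corrected by the actor's starting yaw, then snaps onto it once the time-driven alpha completes.
; RotateToOriginalPoint blends it back to zero relative rotation.
; Each function resets the other's alpha; neither is called within this Blueprint, and RotateEye still prints a debug rotation.
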(event EventBeginPlay
  (Variables|Default|SetRotationPivot (.Yaw (Math|Rotator|BreakRotator (Transformation|GetActorRotation)))))

(event Collision|EventActorBeginOverlap
  (params (OtherActor :type Actor%20Object%20Reference)))

(event EventTick
  (params (DeltaSeconds :type Float%20%28single-precision%29)))

(fn ConstructionScript)

(fn RotateEye
  (params (PlayerPosition :type Vector) (DeltaTime :type Float%20%28single-precision%29))
  (bind _rotationoeil (Variables|Default|GetRotationOeil))
  (bind _rotationpivot (Variables|Default|GetRotationPivot))
  (bind _returnvalue (Transformation|GetWorldLocation _rotationoeil))
  (bind _returnvalue_2 (* -1 _rotationpivot))
  (bind _returnvalue_3 (Math|Rotator|FindLookatRotation _returnvalue PlayerPosition))
  (bind (_roll _pitch _yaw) (Math|Rotator|BreakRotator _returnvalue_3))
  (bind _returnvalue_4 (+ _yaw _returnvalue_2))
  (bind _returnvalue_5 (Math|Rotator|MakeRotator _roll _pitch _returnvalue_4))
  (Transformation|SetRelativeRotation _rotationoeil (Math|Rotator|Lerp(Rotator) (Variables|/Script/Engine.SceneComponent|GetRelativeRotation (Variables|Default|GetRotationOeil)) _returnvalue_5 (Variables|Default|GetAlphaRotationBase) true) false false)
  (Variables|Default|SetAlphaRotationRebase 0.0)
  (if (< (Variables|Default|GetAlphaRotationBase) 1.0)
    (Variables|Default|SetAlphaRotationBase (+ DeltaTime (Variables|Default|GetAlphaRotationBase)))
    (else
      (Development|PrintString (Utilities|String|ToString(Rotator) _returnvalue_5))
      (Transformation|SetRelativeRotation _rotationoeil _returnvalue_5 false false))))

(fn RotatetoOriginalPoint
  (params (DeltaTime :type Float%20%28single-precision%29))
  (Transformation|SetRelativeRotation (Variables|Default|GetRotationOeil) (Math|Rotator|Lerp(Rotator) (Variables|/Script/Engine.SceneComponent|GetRelativeRotation (Variables|Default|GetRotationOeil)) (Math|Rotator|MakeRotator 0.0 0.0 0.0) (Variables|Default|GetAlphaRotationRebase)) false false)
  (if (< (Variables|Default|GetAlphaRotationRebase) 1.0)
    (Variables|Default|SetAlphaRotationRebase (+ DeltaTime (Variables|Default|GetAlphaRotationRebase)))
    (Variables|Default|SetAlphaRotationBase 0.0)))