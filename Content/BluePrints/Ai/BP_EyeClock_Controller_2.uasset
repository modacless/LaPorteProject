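; AI controller for the clock enemy, BP_Enemy_Clock, that makes its eye follow what it sees.
; Sight perception stores any sensed actor as the detected target and clears it when an update reports sight lost.
; Each tick, the controlled pawn rotates its eye toward that target's location, or back to its original point without one.
; A noise-report call is present but never runs.
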(event OnTargetPerceptionUpdated(AIPerceptionSight)
  (params (Actor :type Actor%20Object%20Reference) (Stimulus :type AI%20Stimulus%20Structure))
  (if (Utilities|IsValid Actor)
    (if (.bSuccessfullySensed (Utilities|Struct|BreakAIStimulus Stimulus))
      (Variables|Default|SetPlayerDetect Actor)
      (else
        (Variables|Default|SetPlayerDetect 0)))))

(event EventBeginPlay
  (bind _asbp_enemy_clock (Utilities|Casting|CastToBP_Enemy_Clock (Pawn|GetControlledPawn)))
  (Variables|Default|SetEnemyPawn _asbp_enemy_clock))

(event EventTick
  (params (DeltaSeconds :type Float%20%28single-precision%29))
  (bind _returnvalue (* DeltaSeconds 1.0))
  (bind _enemypawn (Variables|Default|GetEnemyPawn))
  (if (Utilities|IsValid (Variables|Default|GetPlayerDetect))
    (Default|RotateEye _enemypawn (Transformation|GetActorLocation (Variables|Default|GetPlayerDetect)) _returnvalue)
    (else
      (Default|RotatetoOriginalPoint _enemypawn _returnvalue))))

(fn ConstructionScript)