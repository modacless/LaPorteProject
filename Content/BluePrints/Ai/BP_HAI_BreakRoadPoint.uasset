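; BP_HAI_BreakRoadPoint is an AI road point that halts an enemy for a wait time.
; Enter and exit overlaps defer to the parent class, while AiEnterDelay zeroes the BP_HAi controller's walk speed.
; A timeline sized to WaitTime calls StopMovement on every update.
; On finish it sets a hardcoded walk speed rather than the saved BasicSpeed, via a controller lookup that lacks the enemy as input.
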(event EventOnAiExit
  (params (OverlappedComp :type Primitive%20Component%20Object%20Reference) (OtherActor :type Actor%20Object%20Reference) (OtherComp :type Primitive%20Component%20Object%20Reference) (OtherBodyIndex :type Integer))
  (|CallParentFunction OverlappedComp OtherActor OtherComp OtherBodyIndex))

(event EventAiEnterDelay
  (params (OtherActor :type Actor%20Object%20Reference))
  (bind _asbp_hai (Utilities|Casting|CastToBP_HAi OtherActor))
  (bind _ashai_controller (Utilities|Casting|CastToHAI_Controller (AI|GetAIController _asbp_hai)))
  (Variables|Default|SetBasicSpeed (Variables|/Script/LaPorteProject.HAI_Controller|GetEnemyWalkSpeed _ashai_controller))
  (Components|Timeline|SetTimelineLength (Variables|Default|GetWaitTimeLine) (Variables|Default|GetWaitTime))
  (Variables|/Script/LaPorteProject.HAI_Controller|SetEnemyWalkSpeed _ashai_controller 0.0)
  (Timeline|WaitTimeLine PlayFromStart
    (:Update
      (AI|Navigation|StopMovement _ashai_controller))
    (:Finished
      (bind _ashai_controller_2 (Utilities|Casting|CastToHAI_Controller (AI|GetAIController 0)))
      (Variables|/Script/LaPorteProject.HAI_Controller|SetEnemyWalkSpeed _ashai_controller_2 4.5e+02))))

(event EventOnAiEnter
  (params (OverlapComponent :type Primitive%20Component%20Object%20Reference) (OtherActor :type Actor%20Object%20Reference) (OtherComponent :type Primitive%20Component%20Object%20Reference) (OtherBodyIndex :type Integer) (bFromSweep :type Boolean) (SweepResult :type Hit%20Result%20Structure%20%28by%20ref%29))
  (|CallParentFunction OverlapComponent OtherActor OtherComponent OtherBodyIndex bFromSweep SweepResult))

(fn ConstructionScript)