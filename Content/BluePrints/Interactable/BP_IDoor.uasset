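; Interactable door that the player grabs and swings with turn input, with optional key unlocking.
; While held, Tick applies the player's TurnRate to yaw within a locked or open angle limit, with direction set by the player's side.
; On release, a timeline eases the last turn rate to zero for momentum.
; Overlap with the matching BP_Office_Keys swaps in a key mesh and animates it, then clears the lock.
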(event OnComponentBeginOverlap(Box)
  (params (OverlappedComponent :type Primitive%20Component%20Object%20Reference) (OtherActor :type Actor%20Object%20Reference) (OtherComp :type Primitive%20Component%20Object%20Reference) (OtherBodyIndex :type Integer) (bFromSweep :type Boolean) (SweepResult :type Hit%20Result%20Structure%20%28by%20ref%29))
  (bind _keymesh (Variables|Default|GetKeyMesh))
  (bind _relativerotation (Variables|/Script/Engine.SceneComponent|GetRelativeRotation _keymesh))
  (bind (_roll _pitch _yaw) (Math|Rotator|BreakRotator _relativerotation))
  (bind _asbp_office_keys (Utilities|Casting|CastToBP_Office_Keys OtherActor))
  (if (== _asbp_office_keys (Variables|Default|GetKeyToOpen))
    (Rendering|SetVisibility (Variables|/Game/BluePrints/Interactable/BP_Pickable.BP_Pickable_C|GetStaticMesh _asbp_office_keys) false false)
    (Rendering|SetVisibility (Variables|Default|GetKeyMesh) true false)
    (if (> (.X (Math|Vector|BreakVector (Math|Transform|InverseTransformLocation (Transformation|GetActorTransform) (Transformation|GetActorLocation (Game|Player|GetPlayerPawn 0))))) 0.0)
      (Variables|Default|SetSensKeyRotation "0, 0,360.000000")
      (else
        (Transformation|SetRelativeRotation _keymesh (Math|Rotator|MakeRotator _roll (* -1 _pitch) _yaw) false false)
        (Variables|Default|SetSensKeyRotation "0, 0,360.000000")))
    (CallFunction|PlayKeyAnimation)
    (Variables|Default|SetKeyToOpen 0)))

(event Custom|PlayKeyAnimation
  (bind _keymesh (Variables|Default|GetKeyMesh))
  (bind _movemententer (Timeline|KeyAnimation PlayFromStart)
    (:Update
      (Transformation|SetRelativeLocation _keymesh (+ (* (* (Math|Vector|GetUpVector _keymesh) _movemententer) -1) (Variables|/Script/Engine.SceneComponent|GetRelativeLocation _keymesh)) false false)
      (bind _rotationkey (Timeline|KeyRotationAnimation PlayFromStart)
        (:Update
          (Transformation|SetRelativeRotation (Variables|Default|GetkeyPoint) (Math|Rotator|Lerp(Rotator) "0, 0,0.000000" (Variables|Default|GetSensKeyRotation) _rotationkey) false false))
        (:Finished
          (Variables|Default|SetIsLock false))))))

(event EventBeginPlay
  ;[1 1 1] Begin
  (if (Utilities|IsValid (Variables|Default|GetKeyToOpen))
    (Components|StaticMesh|SetStaticMesh (Variables|Default|GetKeyMesh) (Variables|/Script/Engine.StaticMeshComponent|GetStaticMesh (Variables|/Game/BluePrints/Interactable/BP_Pickable.BP_Pickable_C|GetStaticMesh (Variables|Default|GetKeyToOpen))))
    (Rendering|SetVisibility (Variables|Default|GetKeyMesh) false false)))

(event EventTick
  (params (DeltaSeconds :type Float%20%28single-precision%29))
  (bind _returnvalue (Transformation|GetActorRotation))
  (bind _anglemax (Variables|Default|GetAngleMax))
  (bind _yaw (Math|Rotator|BreakRotator _returnvalue))
  ;[1 1 1 1 46] Update
  (if (Variables|Default|GetIsHolding)
    (bind _ashplayer (Utilities|Casting|CastToHPlayer (Game|Player|GetPlayerPawn 0)))
    (if (and (or (< _yaw _anglemax) (< (* (Variables|Default|GetSensToUse) (Variables|/Script/LaPorteProject.HPlayer|GetTurnRate _ashplayer)) 0.0)) (or (> _yaw (* -1 _anglemax)) (> (* (Variables|Default|GetSensToUse) (Variables|/Script/LaPorteProject.HPlayer|GetTurnRate _ashplayer)) 0.0)))
      (Transformation|AddActorLocalRotation (Math|Rotator|MakeRotator 0.0 0.0 (* (Variables|Default|GetSensToUse) (* (Variables|Default|GetSensivity) (Variables|/Script/LaPorteProject.HPlayer|GetTurnRate _ashplayer)))) false false)
      (Variables|Default|SetActualRateDoor (Variables|/Script/LaPorteProject.HPlayer|GetTurnRate _ashplayer)))))

(event EventInterract
  ;[1 1 1 1 58] Use Door
  (if (Variables|Default|GetIsLock)
    (Variables|Default|SetAngleMax (Variables|Default|GetCloseMaxAngle))
    (else
      (Variables|Default|SetAngleMax (Variables|Default|GetOpenMaxAngle))))
  (if (> (.X (Math|Vector|BreakVector (Math|Transform|InverseTransformLocation (Transformation|GetActorTransform) (Transformation|GetActorLocation (Game|Player|GetPlayerPawn 0))))) 0.0)
    (Variables|Default|SetSensToUse 1)
    (else
      (Variables|Default|SetSensToUse -1)))
  (Variables|Default|SetIsHolding true)
  (bind _ashplayer (Utilities|Casting|CastToHPlayer (Game|Player|GetPlayerPawn 0)))
  (Variables|/Script/LaPorteProject.HPlayer|SetPlayerMovement _ashplayer "Use")
  (Variables|/Script/LaPorteProject.HPlayer|SetObjectInHand _ashplayer self))

(event EventStopInterract
  (bind _returnvalue (Transformation|GetActorRotation))
  (bind _actualratedoor (Variables|Default|GetActualRateDoor))
  (bind _yaw (Math|Rotator|BreakRotator _returnvalue))
  ;[1 1 1 1 44] Relase Door
  (Variables|Default|SetIsHolding false)
  (bind _ashplayer (Utilities|Casting|CastToHPlayer (Game|Player|GetPlayerPawn 0)))
  (Variables|/Script/LaPorteProject.HPlayer|SetPlayerMovement _ashplayer "Run")
  (Variables|/Script/LaPorteProject.HPlayer|SetObjectInHand _ashplayer 0)
  (if (!= _actualratedoor 0.0)
    (bind _door (Timeline|CloseDoorTimeLine PlayFromStart)
      (:Update
        (if (< _yaw (Variables|Default|GetAngleMax))
          (if (> _yaw (* -1 (Variables|Default|GetAngleMax)))
            (Transformation|AddActorLocalRotation (Math|Rotator|MakeRotator 0.0 0.0 (* (Variables|Default|GetSensToUse) (Math|Float|Lerp (* _actualratedoor (Variables|Default|GetSensivity)) 0.0 _door))) false false)))))))

(fn ConstructionScript)