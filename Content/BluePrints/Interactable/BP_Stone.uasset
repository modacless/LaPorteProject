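; BP_Stone is an interactable stone that the player can hold and carry.
; Interract and StopInterract toggle an IsHolding flag, which Tick checks each frame.
; While held, the stone teleports without sweep to just in front of the first player pawn along its forward vector.
; The transform is built from location alone, so rotation and scale reset to defaults.
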(event EventInterract
  (Variables|Default|SetIsHolding true))

(event EventStopInterract
  (Variables|Default|SetIsHolding false))

(event EventTick
  (params (DeltaSeconds :type Float%20%28single-precision%29))
  (bind _returnvalue (Game|Player|GetPlayerPawn 0))
  (bind _returnvalue_2 (Transformation|GetActorTransform _returnvalue))
  (bind (_location _rotation) (Math|Transform|BreakTransform _returnvalue_2))
  (if (Variables|Default|GetIsHolding)
    (Transformation|SetActorTransform self (Math|Conversions|ToTransform(Vector) (+ _location (* (Math|Vector|GetForwardVector _rotation) 5.0))) false true)))

(fn ConstructionScript)