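; Pickable, throwable destructible object that the player can carry one at a time.
; Interract, if the player's hand is empty, registers it as ObjectInHand, disables Cube physics and both components' collision, and snaps it to the HoldItem socket.
; StopInterract detaches it, places it ahead of the camera, offset by its bounds plus capsule radius, restores physics and collision, and launches it along the view with an impulse.
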(event EventBeginPlay)

(event Collision|EventActorBeginOverlap
  (params (OtherActor :type Actor%20Object%20Reference)))

(event EventTick
  (params (DeltaSeconds :type Float%20%28single-precision%29)))

(event EventInterract
  (bind _cube (Variables|Default|GetCube))
  (bind _asbp_hplayer (Utilities|Casting|CastToBP_HPlayer (Game|Player|GetPlayerPawn 0)))
  (if (not (Utilities|IsValid (Variables|/Script/LaPorteProject.HPlayer|GetObjectInHand _asbp_hplayer)))
    (Variables|/Script/LaPorteProject.HPlayer|SetObjectInHand _asbp_hplayer self)
    (Physics|SetSimulatePhysics _cube false)
    (Collision|SetCollisionEnabled _cube "NoCollision")
    (Collision|SetCollisionEnabled (Variables|Default|GetDestructible) "NoCollision")
    (Transformation|AttachComponentToComponent (Variables|/Script/Engine.Character|GetMesh _asbp_hplayer) "HoldItem" "SnapToTarget" "SnapToTarget" "KeepRelative" true)))

(event EventStopInterract
  (bind _returnvalue (Game|GetPlayerCameraManager 0))
  (bind _destructible (Variables|Default|GetDestructible))
  (bind _cube (Variables|Default|GetCube))
  (bind _transformcomponent (Variables|/Script/Engine.PlayerCameraManager|GetTransformComponent _returnvalue))
  (bind _returnvalue_2 (Math|Vector|GetForwardVector _transformcomponent))
  (bind _asbp_hplayer (Utilities|Casting|CastToBP_HPlayer (Game|Player|GetPlayerPawn 0)))
  (Variables|/Script/LaPorteProject.HPlayer|SetObjectInHand _asbp_hplayer 0)
  (Transformation|DetachFromActor "KeepRelative" "KeepRelative" "KeepRelative")
  (bind _ashplayer (Utilities|Casting|CastToHPlayer (Game|Player|GetPlayerPawn 0)))
  (Transformation|SetWorldLocation _cube (+ (* _returnvalue_2 (+ (.SphereRadius (Collision|GetComponentBounds (Variables|Default|GetDestructible))) (Variables|/Script/Engine.CapsuleComponent|GetCapsuleRadius (Variables|/Script/Engine.Character|GetCapsuleComponent _ashplayer)))) (Transformation|GetWorldLocation _transformcomponent)) false false)
  (Transformation|SetActorRotation (Math|Conversions|RotationFromXVector (Math|Vector|GetForwardVector (Variables|/Script/Engine.PlayerCameraManager|GetTransformComponent (Variables|/Script/Engine.PlayerController|GetPlayerCameraManager (Game|GetPlayerController 0))))))
  (Physics|SetSimulatePhysics _destructible true)
  (Collision|SetCollisionEnabled _destructible "QueryAndPhysics")
  (Physics|AddImpulse _cube (* _returnvalue_2 1e+04) "None" false))

(fn ConstructionScript)