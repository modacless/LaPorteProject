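; BP_Throwable is an interactable object that launches away from the player's view when interaction stops.
; StopInterract clears the player's ObjectInHand, detaches the actor and moves its mesh in front of the camera, offset by mesh and capsule radii to clear the player.
; It then faces the actor along the camera direction, enables physics and collision, and applies a fixed forward impulse.
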(event EventBeginPlay
  (|CallParentFunction)
  (Collision|SetCollisionEnabled (Variables|Default|GetStaticMesh) "QueryAndPhysics"))

(event EventStopInterract
  (bind _returnvalue (Game|GetPlayerCameraManager 0))
  (bind _staticmesh (Variables|Default|GetStaticMesh))
  (bind _transformcomponent (Variables|/Script/Engine.PlayerCameraManager|GetTransformComponent _returnvalue))
  (bind _returnvalue_2 (Math|Vector|GetForwardVector _transformcomponent))
  (bind _asbp_hplayer (Utilities|Casting|CastToBP_HPlayer (Game|Player|GetPlayerPawn 0)))
  (Variables|/Script/LaPorteProject.HPlayer|SetObjectInHand _asbp_hplayer 0)
  (Transformation|DetachFromActor "KeepRelative" "KeepRelative" "KeepRelative")
  (bind _ashplayer (Utilities|Casting|CastToHPlayer (Game|Player|GetPlayerPawn 0)))
  (Transformation|SetWorldLocation _staticmesh (+ (* _returnvalue_2 (+ (.SphereRadius (Collision|GetComponentBounds (Variables|Default|GetStaticMesh))) (Variables|/Script/Engine.CapsuleComponent|GetCapsuleRadius (Variables|/Script/Engine.Character|GetCapsuleComponent _ashplayer)))) (Transformation|GetWorldLocation _transformcomponent)) false false)
  (Transformation|SetActorRotation (Math|Conversions|RotationFromXVector (Math|Vector|GetForwardVector (Variables|/Script/Engine.PlayerCameraManager|GetTransformComponent (Variables|/Script/Engine.PlayerController|GetPlayerCameraManager (Game|GetPlayerController 0))))))
  (Physics|SetSimulatePhysics _staticmesh true)
  (Collision|SetCollisionEnabled _staticmesh "QueryAndPhysics")
  (Physics|AddImpulse _staticmesh (* _returnvalue_2 1e+04) "None" false))

(fn ConstructionScript
  (|CallParentFunction))