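; Interactable clock that the player winds back by holding it, acting as a timed noise maker.
; Interacting saves the current time, puts the player in Use mode and rewinds on Tick until released.
; It then counts forward at the same doubled speed, rotating the hand pivots to match.
; Once it passes the saved time it stops and rings through a noise event that AI can hear, instigated by the player.
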(event EventBeginPlay
  (CallFunction|SetClockRotation (Variables|Default|GetClockTime)))

(event EventTick
  (params (DeltaSeconds :type Float%20%28single-precision%29))
  (bind _returnvalue (* 2 DeltaSeconds))
  (if (Variables|Default|GetIsholding)
    (CallFunction|RemoveTime _returnvalue)
    (elif (Variables|Default|GetIsCounting)
      (CallFunction|UpdateClock _returnvalue))))

(event EventInterract
  (bind _asbp_hplayer (Utilities|Casting|CastToBP_HPlayer (Game|Player|GetPlayerPawn 0)))
  (Variables|/Script/LaPorteProject.HPlayer|SetPlayerMovement _asbp_hplayer "Use")
  (Variables|/Script/LaPorteProject.HPlayer|SetObjectInHand _asbp_hplayer self)
  (if (Variables|Default|GetIsholding)
    _
    (else
      (Variables|Default|SetClockStartTime (Variables|Default|GetClockTime))))
  (Variables|Default|SetIsholding true)
  (Variables|Default|SetIsCounting true))

(event EventStopInterract
  (Variables|Default|SetIsholding false)
  (bind _ashplayer (Utilities|Casting|CastToHPlayer (Game|Player|GetPlayerPawn 0)))
  (Variables|/Script/LaPorteProject.HPlayer|SetPlayerMovement _ashplayer "Walk")
  (Variables|/Script/LaPorteProject.HPlayer|SetObjectInHand _ashplayer 0))

(fn ConstructionScript)

(fn SetClockRotation
  (params (Time%20to%20set :type F%20Date%20Clock%20Struct%20Structure))
  (bind (_hours _minutes _seconds) (Utilities|Struct|BreakFDateClockStruct Time%20to%20set))
  (Transformation|SetRelativeRotation (Variables|Default|GetClockHandSecondsPivot) (Math|Rotator|MakeRotator (/ (* _seconds 3.6e+02) 6e+01) 0.0 0.0) false false)
  (Transformation|SetRelativeRotation (Variables|Default|GetClockHandMinutesPivot) (Math|Rotator|MakeRotator (/ (* _minutes 3.6e+02) 6e+01) 0.0 0.0) false false)
  (Transformation|SetRelativeRotation (Variables|Default|GetClockHandHoursPivot) (Math|Rotator|MakeRotator (/ (* _hours 3.6e+02) 12.0) 0.0 0.0) false false))

(fn AddTime
  (params (DeltaTime :type Float%20%28single-precision%29))
  (if (> (+ DeltaTime (.Seconds (Utilities|Struct|BreakFDateClockStruct (Variables|Default|GetClockTime)))) 6e+01)
    (if (> (+ (.Minutes (Utilities|Struct|BreakFDateClockStruct (Variables|Default|GetClockTime))) 1.0) 6e+01)
      (if (> (.Hours (Utilities|Struct|BreakFDateClockStruct (Variables|Default|GetClockTime))) 24.0)
        (bind _output_get (Variables|Default|SetClockTime (Utilities|Struct|MakeFDateClockStruct 0.0 0.0 0.0)))
        (CallFunction|SetClockRotation _output_get)
        (else
          (bind _output_get_2 (Variables|Default|SetClockTime (Utilities|Struct|MakeFDateClockStruct (+ (.Hours (Utilities|Struct|BreakFDateClockStruct (Variables|Default|GetClockTime))) 1.0) 0.0 0.0)))
          (CallFunction|SetClockRotation _output_get_2)))
      (else
        (bind _output_get_3 (Variables|Default|SetClockTime (Utilities|Struct|MakeFDateClockStruct (.Hours (Utilities|Struct|BreakFDateClockStruct (Variables|Default|GetClockTime))) (+ (.Minutes (Utilities|Struct|BreakFDateClockStruct (Variables|Default|GetClockTime))) 1.0) 0.0)))
        (CallFunction|SetClockRotation _output_get_3)))
    (else
      (bind _output_get_4 (Variables|Default|SetClockTime (Utilities|Struct|MakeFDateClockStruct (.Hours (Utilities|Struct|BreakFDateClockStruct (Variables|Default|GetClockTime))) (.Minutes (Utilities|Struct|BreakFDateClockStruct (Variables|Default|GetClockTime))) (+ DeltaTime (.Seconds (Utilities|Struct|BreakFDateClockStruct (Variables|Default|GetClockTime)))))))
      (CallFunction|SetClockRotation _output_get_4))))

(fn RemoveTime
  (params (DeltaTime :type Float%20%28single-precision%29))
  (if (< (- (.Seconds (Utilities|Struct|BreakFDateClockStruct (Variables|Default|GetClockTime))) DeltaTime) 0.0)
    (if (< (- (.Minutes (Utilities|Struct|BreakFDateClockStruct (Variables|Default|GetClockTime))) 1.0) 0.0)
      (if (< (.Hours (Utilities|Struct|BreakFDateClockStruct (Variables|Default|GetClockTime))) 0.0)
        (bind _output_get (Variables|Default|SetClockTime (Utilities|Struct|MakeFDateClockStruct 23.0 0.0 0.0)))
        (CallFunction|SetClockRotation _output_get)
        (else
          (bind _output_get_2 (Variables|Default|SetClockTime (Utilities|Struct|MakeFDateClockStruct (- (.Hours (Utilities|Struct|BreakFDateClockStruct (Variables|Default|GetClockTime))) 1.0) 59.0 (.Seconds (Utilities|Struct|BreakFDateClockStruct (Variables|Default|GetClockTime))))))
          (CallFunction|SetClockRotation _output_get_2)))
      (else
        (bind _output_get_3 (Variables|Default|SetClockTime (Utilities|Struct|MakeFDateClockStruct (.Hours (Utilities|Struct|BreakFDateClockStruct (Variables|Default|GetClockTime))) (- (.Minutes (Utilities|Struct|BreakFDateClockStruct (Variables|Default|GetClockTime))) 1.0) 59.0)))
        (CallFunction|SetClockRotation _output_get_3)))
    (else
      (bind _output_get_4 (Variables|Default|SetClockTime (Utilities|Struct|MakeFDateClockStruct (.Hours (Utilities|Struct|BreakFDateClockStruct (Variables|Default|GetClockTime))) (.Minutes (Utilities|Struct|BreakFDateClockStruct (Variables|Default|GetClockTime))) (- (.Seconds (Utilities|Struct|BreakFDateClockStruct (Variables|Default|GetClockTime))) DeltaTime))))
      (CallFunction|SetClockRotation _output_get_4))))

(fn UpdateClock
  (params (DeltaTime :type Float%20%28single-precision%29))
  (bind _clocktime (Variables|Default|GetClockTime))
  (bind _clockstarttime (Variables|Default|GetClockStartTime))
  (bind (_hours _minutes _seconds) (Utilities|Struct|BreakFDateClockStruct _clocktime))
  (bind (_hours_2 _minutes_2 _seconds_2) (Utilities|Struct|BreakFDateClockStruct _clockstarttime))
  (if (Math|Boolean|ANDBoolean (<= _hours _hours_2) (<= _minutes _minutes_2) (<= _seconds _seconds_2))
    (CallFunction|AddTime DeltaTime)
    (else
      (Variables|Default|SetIsCounting false)
      (CallFunction|Ring))))

(fn Ring
  (Class|AISenseHearing|ReportNoiseEvent (Transformation|GetActorLocation) 1.0 (Game|Player|GetPlayerPawn 0) 5e+03 "None"))