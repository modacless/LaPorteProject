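; BP_Stepladder2 is an interactable stepladder that slides along its forward axis when its Interract event fires.
; The event restarts the Moving timeline, whose track value scales a forward step added to ROOT's world location on each update and applied as relative location.
; Pivot and Pivot2 pitch in proportion to ROOT's relative Y position, so they rotate as the ladder travels along that axis.
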(event EventInterract
  (bind _root (Variables|Default|GetROOT))
  (bind _root_2 (Variables|Default|GetROOT))
  (bind _returnvalue (Transformation|GetRelativeTransform _root))
  (bind _location (Math|Transform|BreakTransform _returnvalue))
  (bind _y (Math|Vector|BreakVector _location))
  (bind _returnvalue_2 (* _y 2.0))
  (bind _returnvalue_3 (Math|Rotator|MakeRotator 0.0 _returnvalue_2 0.0))
  (bind _newtrack_0 (Timeline|Moving PlayFromStart)
    (:Update
      (Transformation|SetRelativeLocation (Variables|Default|GetROOT) (+ (* (Math|Vector|GetForwardVector _root_2) (Math|Vector|MakeVector _newtrack_0 _newtrack_0 _newtrack_0)) (Transformation|GetWorldLocation _root_2)) false false)
      (Transformation|SetRelativeRotation (Variables|Default|GetPivot2) _returnvalue_3 false false)
      (Transformation|SetRelativeRotation (Variables|Default|GetPivot) _returnvalue_3 false false))))

(fn ConstructionScript)