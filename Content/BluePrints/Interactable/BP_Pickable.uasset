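; Physics-simulated pickable item that the player can pick up and drop through interaction events.
; Interract stores it as BP_HPlayer's ObjectInHand if the hand is empty, disables physics and collision, and attaches it to the HoldItem socket.
; StopInterract box-traces from the camera using the mesh bounds, then releases it at the hit point or at full interaction range.
; The drop is refused when the hit is too close to the player.
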(event EventBeginPlay
  (Physics|SetSimulatePhysics (Variables|Default|GetStaticMesh) true))

(event EventInterract
  (bind _staticmesh (Variables|Default|GetStaticMesh))
  ;[1 1 1] Pickup
  (bind _asbp_hplayer (Utilities|Casting|CastToBP_HPlayer (Game|Player|GetPlayerPawn 0)))
  (if (not (Utilities|IsValid (Variables|/Script/LaPorteProject.HPlayer|GetObjectInHand _asbp_hplayer)))
    (Variables|/Script/LaPorteProject.HPlayer|SetObjectInHand _asbp_hplayer self)
    (Physics|SetSimulatePhysics _staticmesh false)
    (Collision|SetCollisionEnabled _staticmesh "NoCollision")
    (Transformation|AttachComponentToComponent (Variables|/Script/Engine.Character|GetMesh _asbp_hplayer) "HoldItem" "KeepRelative" "KeepRelative" "KeepRelative" false)
    (Transformation|SetRelativeLocation (Variables|Default|GetStaticMesh) "0, 0, 0" true false)))

(event EventStopInterract
  (bind _returnvalue (Game|GetPlayerCameraManager 0))
  (bind _staticmesh (Variables|Default|GetStaticMesh))
  (bind _staticmesh_2 (Variables|Default|GetStaticMesh))
  (bind _max (Components|StaticMesh|GetLocalBounds _staticmesh_2))
  (bind _transformcomponent (Variables|/Script/Engine.PlayerCameraManager|GetTransformComponent _returnvalue))
  (bind _returnvalue_2 (Transformation|GetWorldLocation _transformcomponent))
  ;[1 1 1] Drop
  (bind _asbp_hplayer (Utilities|Casting|CastToBP_HPlayer (Game|Player|GetPlayerPawn 0)))
  (bind (_outhit _returnvalue_3) (Collision|BoxTraceByChannel _returnvalue_2 (+ _returnvalue_2 (* (Math|Vector|GetForwardVector _transformcomponent) (Variables|/Script/LaPorteProject.HPlayer|GetRangeInterraction _asbp_hplayer))) _max "0, 0, 0" "TraceTypeQuery1" false 0 "None"))
  (if _returnvalue_3
    (Development|PrintString (Utilities|String|ToString(Float) (- (.Distance (Collision|BreakHitResult _outhit)) (Components|Capsule|GetScaledCapsuleRadius (Variables|/Script/Engine.Character|GetCapsuleComponent _asbp_hplayer)))))
    (if (not (< (- (.Distance (Collision|BreakHitResult _outhit)) (Components|Capsule|GetScaledCapsuleRadius (Variables|/Script/Engine.Character|GetCapsuleComponent _asbp_hplayer))) (Math|Vector|VectorLength _max)))
      (Variables|/Script/LaPorteProject.HPlayer|SetObjectInHand _asbp_hplayer 0)
      (Transformation|DetachFromActor "KeepRelative" "KeepRelative" "KeepRelative")
      (Physics|SetSimulatePhysics _staticmesh true)
      (Collision|SetCollisionEnabled _staticmesh "QueryAndPhysics")
      (Transformation|SetWorldLocation _staticmesh (.Location (Collision|BreakHitResult _outhit)) false false))
    (else
      (Variables|/Script/LaPorteProject.HPlayer|SetObjectInHand _asbp_hplayer 0)
      (Transformation|DetachFromActor "KeepRelative" "KeepRelative" "KeepRelative")
      (Physics|SetSimulatePhysics _staticmesh true)
      (Collision|SetCollisionEnabled _staticmesh "QueryAndPhysics")
      (Transformation|SetWorldLocation _staticmesh (+ _returnvalue_2 (* (Math|Vector|GetForwardVector _transformcomponent) (Variables|/Script/LaPorteProject.HPlayer|GetRangeInterraction _asbp_hplayer))) false false))))

(fn ConstructionScript)