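; Trigger box that plays a short scripted cinematic move on the overlapping BP_HPlayer.
; It sets PlayerMovement to Hide, then two chained timelines lerp the player through two marker positions.
; The first timeline also turns the controller toward Position1, while the second's rotation lerp has no alpha input.
; Movement returns to Walk and the DoOnce resets afterwards, while EnableDisableCollider toggles box collision and the disabled flag.
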(event OnComponentBeginOverlap(Box)
  (params (OverlappedComponent :type Primitive%20Component%20Object%20Reference) (OtherActor :type Actor%20Object%20Reference) (OtherComp :type Primitive%20Component%20Object%20Reference) (OtherBodyIndex :type Integer) (bFromSweep :type Boolean) (SweepResult :type Hit%20Result%20Structure%20%28by%20ref%29))
  (if (not (Variables|Default|GetIsDisable))
    (Utilities|FlowControl|DoOnce false
      (:Completed
        (bind _asbp_hplayer (Utilities|Casting|CastToBP_HPlayer OtherActor))
        (bind _output_get (Variables|Default|SetPlayer _asbp_hplayer))
        (Variables|/Script/LaPorteProject.HPlayer|SetPlayerMovement _output_get "Hide")
        (CallFunction|CinematicMovement)))))

(event Custom|CinematicMovement
  (Variables|Default|SetStartRotation (Transformation|GetActorRotation (Game|GetPlayerController 0)))
  (Variables|Default|SetStartPosition (Transformation|GetActorLocation (Variables|Default|GetPlayer)))
  (bind (_direction _position _rotation) (Timeline|ToPosition1 PlayFromStart)
    (:Update
      (Transformation|SetActorLocation (Variables|Default|GetPlayer) (Math|Vector|Lerp(Vector) (Variables|Default|GetStartPosition) (Utilities|Array|Get(acopy) (Variables|Default|GetPositionCinematics)) _position) false false)
      (Transformation|SetActorRotation (Pawn|GetController (Variables|Default|GetPlayer)) (Math|Rotator|Lerp(Rotator) (Variables|Default|GetStartRotation) (Transformation|GetWorldRotation (Variables|Default|GetPosition1)) _rotation)))
    (:Finished
      (Variables|Default|SetStartPosition (Math|Vector|Lerp(Vector) (Variables|Default|GetStartPosition) (Utilities|Array|Get(acopy) (Variables|Default|GetPositionCinematics)) _position))
      (bind _position_2 (Timeline|ToPosition2 PlayFromStart)
        (:Update
          (Transformation|SetActorLocation (Variables|Default|GetPlayer) (Math|Vector|Lerp(Vector) (Variables|Default|GetStartPosition) (Utilities|Array|Get(acopy) (Variables|Default|GetPositionCinematics) 1) _position_2) false false)
          (Transformation|SetActorRotation (Pawn|GetController (Variables|Default|GetPlayer)) (Math|Rotator|Lerp(Rotator) (Variables|Default|GetStartRotation) (Transformation|GetWorldRotation (Variables|Default|GetPosition1)) 0.0)))
        (:Finished
          (Variables|/Script/LaPorteProject.HPlayer|SetPlayerMovement (Variables|Default|GetPlayer) "Walk")
          (Utilities|FlowControl|DoOnce false) ; enters at Reset
        )))))

(event Custom|EnableDisableCollider
  (bind _box (Variables|Default|GetBox))
  (if (Variables|Default|GetIsDisable)
    (Collision|SetCollisionEnabled _box "QueryAndPhysics")
    (Variables|Default|SetIsDisable false)
    (else
      (Collision|SetCollisionEnabled _box "NoCollision")
      (Variables|Default|SetIsDisable true))))

(event EventBeginPlay
  (bind _positioncinematics (Variables|Default|GetPositionCinematics))
  (Utilities|Array|Add _positioncinematics (Transformation|GetWorldLocation (Variables|Default|GetPosition1)))
  (Utilities|Array|Add _positioncinematics (Transformation|GetWorldLocation (Variables|Default|GetPosition2)))
  (Variables|Default|SetIsDisable (Variables|Default|GetDisableOnStart)))

(fn ConstructionScript)