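; BP_Office_Keys is an interactable, pickable office keys actor that extends a parent Blueprint's interaction logic.
; On BeginPlay it applies its SimulatePhysics setting to the static mesh.
; Interacting runs the parent behavior, then breaks the physics constraint to release the keys.
; RotateInDoor zeroes the actor's relative rotation, apparently to align the keys when placed in a door.
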(event EventBeginPlay
  (|CallParentFunction)
  (Physics|SetSimulatePhysics (Variables|Default|GetStaticMesh) (Variables|Default|GetSimulatePhysics)))

(event Collision|EventActorBeginOverlap
  (params (OtherActor :type Actor%20Object%20Reference)))

(event EventInterract
  (|CallParentFunction)
  (Class|PhysicsConstraintComponent|BreakConstraint (Variables|Default|GetPhysicsConstraint)))

(event EventStopInterract
  (|CallParentFunction))

(fn ConstructionScript
  (|CallParentFunction))

(fn RotateinDoor
  (Transformation|SetActorRelativeRotation "0, 0, 0"))