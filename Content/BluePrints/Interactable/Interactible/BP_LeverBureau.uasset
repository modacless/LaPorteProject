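; BP_LeverBureau is an interactable lever that toggles between two states and triggers a linked actor.
; Interract ignores calls while the lever is moving, flips its state, and plays a timeline forward or backward to set PivotLever's world pitch.
; When the timeline finishes, it unlocks the lever, sends ConnectedUseMessage to ActorToUse and reports a noise event at the player pawn's location.
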(event EventBeginPlay)

(event Collision|EventActorBeginOverlap
  (params (OtherActor :type Actor%20Object%20Reference)))

(event EventTick
  (params (DeltaSeconds :type Float%20%28single-precision%29)))

(event EventInterract
  (bind _returnvalue (Game|Player|GetPlayerPawn 0))
  (if (not (Variables|Default|GetIsUsed))
    (Variables|Default|SetIsUsed true)
    (if (Variables|Default|GetStateLever)
      (Variables|Default|SetStateLever false)
      (bind _rotationlever (Timeline|TimeLineLeverRotation ReverseFromEnd)
        (:Update
          (Transformation|SetWorldRotation (Variables|Default|GetPivotLever) (Math|Rotator|MakeRotator 0.0 _rotationlever 0.0) false false))
        (:Finished
          (Variables|Default|SetIsUsed false)
          (Class|ConnectedWire|ConnectedUse(Message) (Variables|Default|GetActorToUse))
          (Class|AISenseHearing|ReportNoiseEvent (Transformation|GetActorLocation _returnvalue) 1.0 _returnvalue 5e+03 "None")))
      (else
        (Variables|Default|SetStateLever true)
        (Timeline|TimeLineLeverRotation PlayFromStart)))))

(fn ConstructionScript)