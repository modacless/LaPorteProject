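; BP_Assiete is a breakable kitchen plate that shatters and makes noise when the player touches it.
; When BP_HPlayer enters its Box, the Destructible component starts simulating physics and takes damage with an upward impulse.
; It reports a long-range noise event for AI hearing at the plate's location, instigated by the player controller.
; The TimeToDeath timeline then serves as a delay before the actor destroys itself.
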(event OnComponentBeginOverlap(Box)
  (params (OverlappedComponent :type Primitive%20Component%20Object%20Reference) (OtherActor :type Actor%20Object%20Reference) (OtherComp :type Primitive%20Component%20Object%20Reference) (OtherBodyIndex :type Integer) (bFromSweep :type Boolean) (SweepResult :type Hit%20Result%20Structure%20%28by%20ref%29))
  (bind _destructible (Variables|Default|GetDestructible))
  (bind _returnvalue (Transformation|GetWorldLocation _destructible))
  (Utilities|Casting|CastToBP_HPlayer OtherActor)
  (Physics|SetSimulatePhysics _destructible true)
  (Class|DestructibleComponent|ApplyDamage _destructible 1e+01 _returnvalue (* (Math|Vector|VectorUp) 100) 1e+01)
  (Class|AISenseHearing|ReportNoiseEvent _returnvalue 1.0 (Game|GetPlayerController 0) 5e+04 "None")
  (Timeline|TimeToDeath PlayFromStart
    (:Finished
      (Actor|DestroyActor))))

(event EventBeginPlay
  (|CallParentFunction) ; This node is disabled and will not be called.\nDrag off pins to build functionality.
)

(event Collision|EventActorBeginOverlap
  (params (OtherActor :type Actor%20Object%20Reference)))

(event EventTick
  (params (DeltaSeconds :type Float%20%28single-precision%29)))

(fn ConstructionScript
  (|CallParentFunction))