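; Kitchen event actor that makes a book fall and create noise, judging by its name and logic.
; StartEvent enables physics simulation on its own static mesh and on the mesh of a referenced ActorToPush.
; When its box overlaps an actor tagged Ground, it reports a long-range AI noise at the mesh location, instigated by the player pawn, and prints a debug string.
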(event OnComponentBeginOverlap(Box)
  (params (OverlappedComponent :type Primitive%20Component%20Object%20Reference) (OtherActor :type Actor%20Object%20Reference) (OtherComp :type Primitive%20Component%20Object%20Reference) (OtherBodyIndex :type Integer) (bFromSweep :type Boolean) (SweepResult :type Hit%20Result%20Structure%20%28by%20ref%29))
  (if (Actor|ActorHasTag OtherActor "Ground")
    (bind _asbp_hplayer (Utilities|Casting|CastToBP_HPlayer (Game|Player|GetPlayerPawn 0)))
    (Class|AISenseHearing|ReportNoiseEvent (Transformation|GetWorldLocation (Variables|Default|GetStaticMesh)) 1.0 _asbp_hplayer 5e+04 "None")
    (Development|PrintString "Sound")))

(event EventBeginPlay)

(event Collision|EventActorBeginOverlap
  (params (OtherActor :type Actor%20Object%20Reference)))

(event EventTick
  (params (DeltaSeconds :type Float%20%28single-precision%29)))

(event EventStartEvent
  (Physics|SetSimulatePhysics (Variables|Default|GetStaticMesh) true)
  (Physics|SetSimulatePhysics (Variables|/Game/BluePrints/Interactable/BP_Pickable.BP_Pickable_C|GetStaticMesh (Variables|Default|GetActorToPush)) true))

(fn ConstructionScript)