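; BP_Clock is an interactable clock whose second, minute and hour hands track a simulated time running at a configurable speed.
; Tick normally advances ClockTime through UpdateTime, which rotates the hand meshes via SetClockTimeRotation.
; Interacting makes Tick run ResetRotation three times per frame instead, winding each hand the shorter way toward zero.
; Once seconds and minutes near zero (hours go unchecked), it rings and resumes ticking; audio completion sets AudioFinished.
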(event OnAudioFinished(ClockRingCue)
  (Variables|Default|SetAudioFinished true))

(event EventTick
  (params (DeltaSeconds :type Float%20%28single-precision%29))
  (bind _returnvalue (* DeltaSeconds 1e+01))
  (bind _clocktime (Variables|Default|GetClockTime))
  (if (Variables|Default|GetIsActivate)
    (CallFunction|ResetRotation _returnvalue _clocktime)
    (CallFunction|ResetRotation _returnvalue _clocktime)
    (CallFunction|ResetRotation _returnvalue _clocktime)
    (else
      (CallFunction|UpdateTime (* DeltaSeconds (Variables|Default|GetTimePerSecondToMult))))))

(event EventInterract
  (Variables|Default|SetIsActivate true))

(event EventBeginPlay
  (CallFunction|SetClockTimeRotation (Variables|Default|GetClockTime))
  (Audio|Components|Audio|Stop (Variables|Default|GetClockRingCue)))

(fn ConstructionScript)

(fn Ring
  (Audio|Components|Audio|Play (Variables|Default|GetClockRingCue) 0.0))

(fn SetClockTimeRotation
  (params (Time :type F%20Date%20Clock%20Struct%20Structure))
  (bind (_hours _minutes _seconds) (Utilities|Struct|BreakFDateClockStruct Time))
  (Transformation|SetWorldRotation (Variables|Default|GetSecondMesh) (Math|Rotator|MakeRotator 0.0 (/ (* _seconds 3.6e+02) 6e+01) 0.0) false false)
  (Transformation|SetWorldRotation (Variables|Default|GetMinutesMesh) (Math|Rotator|MakeRotator 0.0 (/ (* _minutes 3.6e+02) 6e+01) 0.0) false false)
  (Transformation|SetWorldRotation (Variables|Default|GetHourMesh) (Math|Rotator|MakeRotator 0.0 (/ (* _hours 3.6e+02) 12.0) 0.0) false false))

(fn UpdateTime
  (params (DeltaTime :type Float%20%28single-precision%29))
  (if (> (+ DeltaTime (.Seconds (Utilities|Struct|BreakFDateClockStruct (Variables|Default|GetClockTime)))) 6e+01)
    (if (> (+ (.Minutes (Utilities|Struct|BreakFDateClockStruct (Variables|Default|GetClockTime))) 1.0) 6e+01)
      (if (> (.Hours (Utilities|Struct|BreakFDateClockStruct (Variables|Default|GetClockTime))) 24.0)
        (bind _output_get (Variables|Default|SetClockTime (Utilities|Struct|MakeFDateClockStruct 0.0 0.0 0.0)))
        (CallFunction|SetClockTimeRotation _output_get)
        (else
          (bind _output_get_2 (Variables|Default|SetClockTime (Utilities|Struct|MakeFDateClockStruct (+ (.Hours (Utilities|Struct|BreakFDateClockStruct (Variables|Default|GetClockTime))) 1.0) 0.0 0.0)))
          (CallFunction|SetClockTimeRotation _output_get_2)))
      (else
        (bind _output_get_3 (Variables|Default|SetClockTime (Utilities|Struct|MakeFDateClockStruct (.Hours (Utilities|Struct|BreakFDateClockStruct (Variables|Default|GetClockTime))) (+ (.Minutes (Utilities|Struct|BreakFDateClockStruct (Variables|Default|GetClockTime))) 1.0) 0.0)))
        (CallFunction|SetClockTimeRotation _output_get_3)))
    (else
      (bind _output_get_4 (Variables|Default|SetClockTime (Utilities|Struct|MakeFDateClockStruct (.Hours (Utilities|Struct|BreakFDateClockStruct (Variables|Default|GetClockTime))) (.Minutes (Utilities|Struct|BreakFDateClockStruct (Variables|Default|GetClockTime))) (+ DeltaTime (.Seconds (Utilities|Struct|BreakFDateClockStruct (Variables|Default|GetClockTime)))))))
      (CallFunction|SetClockTimeRotation _output_get_4))))

(fn ResetRotation
  (params (DeltaTime :type Float%20%28single-precision%29) (FTime :type F%20Date%20Clock%20Struct%20Structure))
  (bind (_hours _minutes _seconds) (Utilities|Struct|BreakFDateClockStruct FTime))
  (Utilities|FlowControl|Sequence
    (:then_0
      (if (< _seconds 3e+01)
        (bind _output_get (LocalVariables|SetSeconds (- _seconds DeltaTime)))
        (if (< _output_get 0.0)
          (LocalVariables|SetSeconds 0.0))
        (else
          (bind _output_get_2 (LocalVariables|SetSeconds (+ _seconds DeltaTime)))
          (if (> _output_get_2 6e+01)
            (LocalVariables|SetSeconds 0.0)))))
    (:then_1
      (if (< _minutes 3e+01)
        (bind _output_get_3 (LocalVariables|SetMinutes (- _minutes DeltaTime)))
        (if (< _output_get_3 0.0)
          (LocalVariables|SetMinutes 0.0))
        (else
          (bind _output_get_4 (LocalVariables|SetMinutes (+ _minutes DeltaTime)))
          (if (> _output_get_4 6e+01)
            (LocalVariables|SetMinutes 0.0)))))
    (:then_2
      (if (< _hours 12.0)
        (bind _output_get_5 (LocalVariables|SetHours (- _hours DeltaTime)))
        (if (< _output_get_5 0.0)
          (LocalVariables|SetHours 0.0))
        (else
          (bind _output_get_6 (LocalVariables|SetHours (+ _hours DeltaTime)))
          (if (> _output_get_6 24.0)
            (LocalVariables|SetHours 0.0))))
      (bind _output_get_7 (Variables|Default|SetClockTime (Utilities|Struct|MakeFDateClockStruct (LocalVariables|GetHours) (LocalVariables|GetMinutes) (LocalVariables|GetSeconds))))
      (CallFunction|SetClockTimeRotation _output_get_7)
      (if (Math|Boolean|ANDBoolean (Math|Float|NearlyEqual(Float) (LocalVariables|GetSeconds) 0.0 0.1) (Math|Float|NearlyEqual(Float) (LocalVariables|GetMinutes) 0.0 0.1) (Math|Float|NearlyEqual(Float) (LocalVariables|GetMinutes) 0.0 0.1))
        (Variables|Default|SetIsActivate false)
        (CallFunction|Ring)))))