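; BP_Ladder is an interactable ladder that lets BP_HPlayer climb.
; A box overlap tracks when the player is in range, and Interract then snaps them to ForwardPoint or BehindPoint based on their side in local X, nudging the front snap by the mesh forward vector.
; It switches the player to Climb with Flying movement and stores itself as ObjectInHand.
; StopInterract restores walking and clears that reference.
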(event OnComponentBeginOverlap(Box)
  (params (OverlappedComponent :type Primitive%20Component%20Object%20Reference) (OtherActor :type Actor%20Object%20Reference) (OtherComp :type Primitive%20Component%20Object%20Reference) (OtherBodyIndex :type Integer) (bFromSweep :type Boolean) (SweepResult :type Hit%20Result%20Structure%20%28by%20ref%29))
  (Utilities|Casting|CastToBP_HPlayer OtherActor)
  (Variables|Default|SetIsInLadderZone true))

(event OnComponentEndOverlap(Box)
  (params (OverlappedComponent :type Primitive%20Component%20Object%20Reference) (OtherActor :type Actor%20Object%20Reference) (OtherComp :type Primitive%20Component%20Object%20Reference) (OtherBodyIndex :type Integer))
  (Utilities|Casting|CastToBP_HPlayer OtherActor)
  (Variables|Default|SetIsInLadderZone false))

(event EventInterract
  (bind _returnvalue (Game|Player|GetPlayerPawn 0))
  (bind _meshladder (Variables|Default|GetMeshLadder))
  (bind _forwardpoint (Variables|Default|GetForwardPoint))
  (bind _behindpoint (Variables|Default|GetBehindPoint))
  (bind _returnvalue_2 (Transformation|GetWorldLocation _behindpoint))
  (bind _returnvalue_3 (Math|Vector|GetForwardVector _meshladder))
  (bind _returnvalue_4 (Transformation|GetWorldLocation _forwardpoint))
  (bind (_x _y _z) (Math|Vector|BreakVector _returnvalue_2))
  (bind _returnvalue_5 (+ _returnvalue_3 _returnvalue_4))
  (bind (_x_2 _y_2 _z_2) (Math|Vector|BreakVector _returnvalue_5))
  (if (Variables|Default|GetIsInLadderZone)
    (if (> (.X (Math|Vector|BreakVector (Math|Transform|InverseTransformLocation (Transformation|GetActorTransform) (Transformation|GetActorLocation (Game|Player|GetPlayerPawn 0))))) 0.0)
      (Transformation|SetActorLocation _returnvalue (Math|Vector|MakeVector _x_2 _y_2 _z_2) false false)
      (else
        (Transformation|SetActorLocation (Game|Player|GetPlayerPawn 0) (Math|Vector|MakeVector _x _y _z) false false)))
    (bind _asbp_hplayer (Utilities|Casting|CastToBP_HPlayer _returnvalue))
    (Variables|/Script/LaPorteProject.HPlayer|SetPlayerMovement _asbp_hplayer "Climb")
    (Variables|/Script/LaPorteProject.HPlayer|SetObjectInHand _asbp_hplayer self)
    (Pawn|Components|CharacterMovement|SetMovementMode (Variables|/Script/Engine.Character|GetCharacterMovement _asbp_hplayer) "MOVE_Flying" 0)
    (Components|Movement|StopMovementImmediately (Variables|/Script/Engine.Character|GetCharacterMovement _asbp_hplayer))))

(event EventStopInterract
  (bind _asbp_hplayer (Utilities|Casting|CastToBP_HPlayer (Game|Player|GetPlayerPawn 0)))
  (if (Utilities|Enum|Equal(Enum) (Variables|/Script/LaPorteProject.HPlayer|GetPlayerMovement _asbp_hplayer) "Climb")
    (Variables|/Script/LaPorteProject.HPlayer|SetPlayerMovement _asbp_hplayer "Walk")
    (Variables|/Script/LaPorteProject.HPlayer|SetObjectInHand _asbp_hplayer 0)
    (Pawn|Components|CharacterMovement|SetMovementMode (Variables|/Script/Engine.Character|GetCharacterMovement _asbp_hplayer) "MOVE_Walking" 0)))

(fn ConstructionScript)