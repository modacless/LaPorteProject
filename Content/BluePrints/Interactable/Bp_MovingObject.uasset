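; An interactable moving object that slides its mesh back and forth by an offset vector each time it is used.
; Interact is ignored while moving, otherwise it toggles an on/off switch and calls MovingOn or MovingOff, which share the same logic.
; A timeline lerps the mesh from its start location, then negates the offset and stores the new start, so the next use reverses the move.
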(event Custom|MovingOn
  (Variables|Default|SetisMoving true)
  (bind _alpha (Timeline|MovementOn PlayFromStart)
    (:Update
      (Transformation|SetWorldLocation (Variables|Default|GetMesh) (Math|Vector|Lerp(Vector) (Variables|Default|GetStartLocation) (+ (Variables|Default|GetStartLocation) (Variables|Default|GetMouvement%20Direction)) _alpha) false false))
    (:Finished
      (Variables|Default|SetMouvement%20Direction (* (Variables|Default|GetMouvement%20Direction) -1.0))
      (Variables|Default|SetisMoving false)
      (Variables|Default|SetStartLocation (Transformation|GetWorldLocation (Variables|Default|GetMesh))))))

(event Custom|MovingOff
  (Variables|Default|SetisMoving true)
  (bind _alpha (Timeline|MovementOn PlayFromStart)
    (:Update
      (Transformation|SetWorldLocation (Variables|Default|GetMesh) (Math|Vector|Lerp(Vector) (Variables|Default|GetStartLocation) (+ (Variables|Default|GetStartLocation) (Variables|Default|GetMouvement%20Direction)) _alpha) false false))
    (:Finished
      (Variables|Default|SetMouvement%20Direction (* (Variables|Default|GetMouvement%20Direction) -1.0))
      (Variables|Default|SetisMoving false)
      (Variables|Default|SetStartLocation (Transformation|GetWorldLocation (Variables|Default|GetMesh))))))

(event EventInterract
  (if (not (Variables|Default|GetisMoving))
    (if (Variables|Default|GetOnOffSwitch)
      (Variables|Default|SetOnOffSwitch false)
      (CallFunction|MovingOff)
      (else
        (Variables|Default|SetOnOffSwitch true)
        (CallFunction|Movingon)))))

(event EventBeginPlay
  (Variables|Default|SetStartLocation (Transformation|GetWorldLocation (Variables|Default|GetMesh))))

(fn ConstructionScript)