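; Wardrobe hiding spot that the player enters or leaves by interacting while inside its trigger.
; Interract checks the player's movement state, swings both doors via a timeline, then calls HidePlayer or FreePlayer to switch state and blend the view.
; When the swing ends, the hidden pawn moves to the wardrobe camera, or a freed pawn, already returned to its saved location, becomes visible.
; Separate OpenDoor/CloseDoor events only set zero yaw.
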(event OnComponentBeginOverlap(CollisionTrigger)
  (params (OverlappedComponent :type Primitive%20Component%20Object%20Reference) (OtherActor :type Actor%20Object%20Reference) (OtherComp :type Primitive%20Component%20Object%20Reference) (OtherBodyIndex :type Integer) (bFromSweep :type Boolean) (SweepResult :type Hit%20Result%20Structure%20%28by%20ref%29))
  (Utilities|Casting|CastToHPlayer OtherActor)
  (Variables|Default|SetCanOpen true))

(event OnComponentEndOverlap(CollisionTrigger)
  (params (OverlappedComponent :type Primitive%20Component%20Object%20Reference) (OtherActor :type Actor%20Object%20Reference) (OtherComp :type Primitive%20Component%20Object%20Reference) (OtherBodyIndex :type Integer))
  (Utilities|Casting|CastToHPlayer OtherActor)
  (Variables|Default|SetCanOpen false))

(event Custom|HidePlayer
  (bind _returnvalue (Game|GetPlayerController 0))
  (bind _returnvalue_2 (Game|Player|GetPlayerPawn 0))
  ;[1 1 1 1 36] Hide/Unhide
  (Variables|Default|SetOldLocation (Transformation|GetWorldLocation (Variables|/Script/Engine.Actor|GetRootComponent (Game|Player|GetPlayerPawn 0))))
  (bind _ashplayer (Utilities|Casting|CastToHPlayer (Game|GetPlayerCharacter 0)))
  (Variables|/Script/LaPorteProject.HPlayer|SetPlayerMovement _ashplayer "Hide")
  (Input|DisableInput _returnvalue)
  (bind _ashplayer_controller (Utilities|Casting|CastToHPlayer_Controller _returnvalue))
  (Collision|SetActorEnableCollision _ashplayer_controller false)
  (Game|Player|SetViewTargetwithBlend _returnvalue self 0.5 "VTBlend_Linear" 0.0 false)
  (Rendering|SetActorHiddenInGame _returnvalue_2 true)
  (bind _asbp_hplayer (Utilities|Casting|CastToBP_HPlayer _returnvalue_2))
  (Variables|/Script/LaPorteProject.HPlayer|SetIsHide _asbp_hplayer true))

(event Custom|RotateDoor
  (bind _returnvalue (Game|Player|GetPlayerPawn 0))
  ;[1 1 1 1 36] RotateDoor
  (bind _zrot (Timeline|RotateTimeline PlayFromStart)
    (:Update
      (Utilities|FlowControl|Sequence
        (:then_0
          (Transformation|SetRelativeRotation (Variables|Default|GetRotationLeft) (Math|Rotator|MakeRotator 0.0 0.0 (* -1 _zrot)) false false))
        (:then_1
          (Transformation|SetRelativeRotation (Variables|Default|GetRotationRight) (Math|Rotator|MakeRotator 0.0 0.0 _zrot) false false))))
    (:Finished
      (bind _ashplayer (Utilities|Casting|CastToHPlayer _returnvalue))
      (if (Utilities|Enum|Equal(Enum) (Variables|/Script/LaPorteProject.HPlayer|GetPlayerMovement _ashplayer) "Hide")
        (Transformation|SetActorLocation _returnvalue (Transformation|GetWorldLocation (Variables|Default|GetCamera)) false false)
        (else
          (Rendering|SetActorHiddenInGame (Game|Player|GetPlayerPawn 0) false))))))

(event Custom|FreePlayer
  (bind _returnvalue (Game|GetPlayerController 0))
  ;[1 1 1 1 36] Hide/Unhide
  (Transformation|SetActorLocation (Game|Player|GetPlayerPawn 0) (Variables|Default|GetOldLocation) false true)
  (bind _ashplayer (Utilities|Casting|CastToHPlayer (Game|GetPlayerCharacter 0)))
  (Variables|/Script/LaPorteProject.HPlayer|SetPlayerMovement _ashplayer "Walk")
  (Input|EnableInput _returnvalue)
  (bind _ashplayer_controller (Utilities|Casting|CastToHPlayer_Controller _returnvalue))
  (Collision|SetActorEnableCollision _ashplayer_controller true)
  (Game|Player|SetViewTargetwithBlend _returnvalue _returnvalue 0.5 "VTBlend_Linear" 0.0 false)
  (bind _asbp_hplayer (Utilities|Casting|CastToBP_HPlayer (Game|Player|GetPlayerPawn 0)))
  (Variables|/Script/LaPorteProject.HPlayer|SetIsHide _asbp_hplayer true))

(event Custom|OpenDoor
  ;[1 1 1 1 36] OpenDoor
  (Timeline|OpenDoorTimeLine PlayFromStart
    (:Update
      (Utilities|FlowControl|Sequence
        (:then_0
          (Transformation|SetRelativeRotation (Variables|Default|GetRotationLeft) (Math|Rotator|MakeRotator 0.0 0.0 (* -1 0.0)) false false))
        (:then_1
          (Transformation|SetRelativeRotation (Variables|Default|GetRotationRight) (Math|Rotator|MakeRotator 0.0 0.0 0.0) false false))))
    (:Finished
      (Variables|Default|SetDoorOpen true))))

(event Custom|CloseDoor
  ;[1 1 1 1 36] ClooseDoor
  (if (Variables|Default|GetDoorOpen)
    (Timeline|CloseDoorTimeLine ReverseFromEnd
      (:Update
        (Utilities|FlowControl|Sequence
          (:then_0
            (Transformation|SetRelativeRotation (Variables|Default|GetRotationLeft) (Math|Rotator|MakeRotator 0.0 0.0 (* -1 0.0)) false false))
          (:then_1
            (Transformation|SetRelativeRotation (Variables|Default|GetRotationRight) (Math|Rotator|MakeRotator 0.0 0.0 0.0) false false))))
      (:Finished
        (Variables|Default|SetDoorOpen false)))))

(event EventInterract
  (if (Variables|Default|GetCanOpen)
    (bind _ashplayer (Utilities|Casting|CastToHPlayer (Game|GetPlayerCharacter 0)))
    (if (Utilities|Enum|Equal(Enum) (Variables|/Script/LaPorteProject.HPlayer|GetPlayerMovement _ashplayer) "Hide")
      (CallFunction|RotateDoor)
      (CallFunction|FreePlayer)
      (else
        (CallFunction|RotateDoor)
        (CallFunction|HidePlayer)))))

(fn ConstructionScript)